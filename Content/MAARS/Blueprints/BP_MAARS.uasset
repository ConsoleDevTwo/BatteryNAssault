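; BP_MAARS is a player-controlled tracked robot with a rotating weapon tower, spring-arm zoom and repaintable body color.
; Movement is physics-driven, using angular velocity to turn and a speed-limited force along a direction blended from a ground box trace.
; Input-fed engine speed and acceleration drive track material tiling, the AnimBP and engine audio, while tower angles also feed the AnimBP.
; Holding Fire loops a timer spawning projectiles, effects and ejected physics clips from weapon sockets.
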(event Custom|UpdateAiming
  (bind _springarm (Variables|Default|GetSpringArm))
  ;[1 1 1] Aiming
  (Variables|/Script/Engine.SpringArmComponent|SetTargetArmLength _springarm (Math|Float|Lerp (Variables|/Script/Engine.SpringArmComponent|GetTargetArmLength _springarm) (Variables|Cache|GetTargetArmLen) 0.16)))

(event Custom|UpdateEngineSound
  (bind _enginesound (Variables|Default|GetEngineSound))
  (bind _engineaccel (Variables|Cache|GetEngineAccel))
  (bind _returnvalue (/ _engineaccel 12.0))
  (bind _returnvalue_2 (Math|Float|Clamp(Float) _returnvalue 0.1))
  ;[1 1 1] Engine Sounds
  (if (== _engineaccel 0.0)
    (Audio|Components|Audio|Stop _enginesound)
    (else
      (if (Audio|Components|Audio|IsPlaying _enginesound)
        _
        (else
          (Audio|Components|Audio|Play _enginesound 0.0)))
      (Audio|Components|Audio|SetPitchMultiplier _enginesound _returnvalue_2)
      (Audio|Components|Audio|SetVolumeMultiplier _enginesound _returnvalue_2 :!class /Script/Engine.AudioComponent))))

(event Custom|UpdateSkControlsAndMats
  ;[1 1 1] Update Skeletal Controls and Material
  (Rendering|Material|SetScalarParameterValue (Variables|Cache|GetM_Tracks) "TilingSpeed" (* (Variables|Cache|GetEngineSpeed) -0.1) :!class /Script/Engine.MaterialInstanceDynamic)
  (bind _asanim_bp_maars (Utilities|Casting|CastToAnimBP_MAARS (Components|SkeletalMesh|GetAnimInstance (Variables|Default|GetMesh))))
  (Variables|/Game/MAARS/Blueprints/AnimBP_MAARS.AnimBP_MAARS_C|SetSpeed _asanim_bp_maars (Variables|Cache|GetEngineSpeed))
  (Variables|/Game/MAARS/Blueprints/AnimBP_MAARS.AnimBP_MAARS_C|SetTowerRot_X _asanim_bp_maars (Variables|Cache|GetTowerRotation_X))
  (Variables|/Game/MAARS/Blueprints/AnimBP_MAARS.AnimBP_MAARS_C|SetTowerRot_Y _asanim_bp_maars (Variables|Cache|GetTowerRotation_Y)))

(event Custom|SpawnProjectile
  (bind _weapon (Variables|Default|GetWeapon))
  (bind _weapon_2 (Variables|Default|GetWeapon))
  (bind _returnvalue (Transformation|GetSocketTransform _weapon_2 "ClipPoint" "RTS_World"))
  (bind _returnvalue_2 (Transformation|GetSocketTransform _weapon "FirePoint" "RTS_World"))
  (bind (_location _rotation) (Math|Transform|BreakTransform _returnvalue_2))
  ;[1 1 1] Fire Logic
  (Audio|SpawnSoundAttached "/Game/MAARS/Sounds/S_Shot_Cue.S_Shot_Cue" (VehicleSound|GetRootComponent))
  (Game|SpawnActorfromClass "/Game/MAARS/Blueprints/BP_MAARS_Projectile.BP_MAARS_Projectile_C" _returnvalue_2 "AlwaysSpawn" 0 0)
  (Effects|SpawnEmitteratLocation "/Game/MAARS/Particles/P_ProjFire.P_ProjFire" _location _rotation)
  (bind _returnvalue_3 (Game|SpawnActorfromClass "/Game/MAARS/Blueprints/BP_Clip.BP_Clip_C" _returnvalue "AlwaysSpawn" 0 0))
  (Physics|AddImpulse (Variables|/Game/MAARS/Blueprints/BP_Clip.BP_Clip_C|GetClipMesh _returnvalue_3) (Math|Transform|TransformDirection _returnvalue (* (Math|Vector|MakeVector (Math|Random|RandomFloatinRange -15.0 15.0) (Math|Random|RandomFloatinRange 8e+01 1.3e+02) (Math|Random|RandomFloatinRange 3e+01 8e+01)) 4.0)) "None" false))

(event Custom|AddEngineSpeed
  (params (dSpeed :type Float%20%28single-precision%29) (dMul :type Float%20%28single-precision%29))
  ;[1 1 1] Engine Speed & Accel
  (Variables|Cache|SetEngineSpeed (+ (* dSpeed dMul) (Variables|Cache|GetEngineSpeed)))
  (Variables|Cache|SetEngineAccel (Math|Float|Clamp(Float) (- (+ (Variables|Cache|GetEngineAccel) (* (Math|Float|Absolute(Float) dSpeed) 0.4)) 0.1) 0.0 12.0)))

(event Custom|AddMovement
  (params (AForce :type Vector))
  ;[1 1 1] Updating movement
  (if (not (> (Math|Vector|VectorLength (Transformation|GetVelocity)) (Variables|Const|GetMaxVelocity)))
    (Physics|AddForce (CallFunction|GetRootMesh) AForce "None" false)))

(event EventBeginPlay)

(event Collision|EventActorBeginOverlap
  (params (OtherActor :type Actor%20Object%20Reference)))

(event EventTick
  (params (DeltaSeconds :type Float%20%28single-precision%29))
  ;[1 1 1] Tick
  (Utilities|FlowControl|Sequence
    (:then_0
      (CallFunction|UpdateSkControlsandMats))
    (:then_1
      (CallFunction|UpdateEngineSound))
    (:then_2
      (CallFunction|UpdateAiming))))

(event Input|ActionEvents|InputActionZoom
  (params (Key :type Key%20Structure :default "AnyKey"))
  ;[1 1 1] Aiming
  (:Pressed
    (Variables|Cache|SetTargetArmLen 1e+02))
  (:Released
    (Variables|Cache|SetTargetArmLen 3e+02)))

(event Input|ActionEvents|InputActionFire
  (params (Key :type Key%20Structure :default "AnyKey"))
  ;[1 1 1] Fire Logic
  (:Pressed
    (if (Variables|Const|GetbCanFire)
      (bind _returnvalue (Utilities|Time|SetTimerbyFunctionName 0 "SpawnProjectile" (Variables|Const|GetReFireDelay) true))
      (Variables|Cache|SetSpawnProjectileTimer _returnvalue)))
  (:Released
    (Class|KismetSystemLibrary|ClearTimerHandle (Variables|Cache|GetSpawnProjectileTimer))))

(event Input|AxisEvents|InputAxisTurn
  (params (AxisValue :type Float%20%28single-precision%29))
  ;[1 1 1] Movement
  (Variables|Cache|SetTowerRotation_X (+ AxisValue (Variables|Cache|GetTowerRotation_X))))

(event Input|AxisEvents|InputAxisMoveForward
  (params (AxisValue :type Float%20%28single-precision%29))
  ;[1 1 1] Movement
  (if (== (stale Input|AxisEvents|InputAxisMoveRight AxisValue) 0.0)
    (CallFunction|AddMovement (* (CallFunction|GetMovementVector) (* AxisValue (Variables|Const|GetMovSpeed))))
    (CallFunction|AddEngineSpeed AxisValue -0.05)))

(event Input|AxisEvents|InputAxisMoveRight
  (params (AxisValue :type Float%20%28single-precision%29))
  ;[1 1 1] Movement
  (Class|PrimitiveComponent|SetPhysicsAngularVelocity (CallFunction|GetRootMesh) (Math|Vector|MakeVector 0.0 0.0 (* AxisValue (* (Utilities|Time|GetWorldDeltaSeconds) (Variables|Const|GetRotSpeed)))) false "None")
  (CallFunction|AddEngineSpeed AxisValue -0.03))

(event Input|AxisEvents|InputAxisView
  (params (AxisValue :type Float%20%28single-precision%29))
  ;[1 1 1] Movement
  (Variables|Cache|SetTowerRotation_Y (Math|Float|Clamp(Float) (+ AxisValue (Variables|Cache|GetTowerRotation_Y)) (Variables|Const|GetTowerRotationY_Min) (Variables|Const|GetTowerRotationY_Max))))

(fn ConstructionScript
  (bind _returnvalue (Class|KismetSystemLibrary|MakeLiteralInteger))
  (bind _returnvalue_2 (Class|KismetSystemLibrary|MakeLiteralInteger 1))
  (Utilities|FlowControl|Sequence
    (:then_0
      ;[1 1 1] Attach weapon
      (Class|SceneComponent|Attachto (Variables|Default|GetWeapon) (Variables|Default|GetMesh) "S_WEAPON" "KeepRelativeOffset" true))
    (:then_1
      ;[1 1 1] Attach glass
      (Class|SceneComponent|Attachto (Variables|Default|GetMaars_Glass) (Variables|Default|GetMesh) "S_WEAPON" "KeepRelativeOffset" true))
    (:then_2
      ;[1 1 1] Get material 0
      (Utilities|IsValid (Variables|Cache|GetM_Main)
        (:Is%20Not%20Valid
          (bind _returnvalue_3 (Rendering|Material|CreateDynamicMaterialInstance (Rendering|Material|GetMaterial (Variables|Default|GetMesh) _returnvalue) :!class /Script/Engine.KismetMaterialLibrary))
          (bind _output_get (Variables|Cache|SetM_Main _returnvalue_3))
          (Rendering|Material|SetMaterial (Variables|Default|GetMesh) _returnvalue _output_get)
          ;[1 1 1] Get material 1
          (Utilities|IsValid (Variables|Cache|GetM_Tracks)
            (:Is%20Not%20Valid
              (bind _returnvalue_4 (Rendering|Material|CreateDynamicMaterialInstance (Rendering|Material|GetMaterial (Variables|Default|GetMesh) _returnvalue_2) :!class /Script/Engine.KismetMaterialLibrary))
              (bind _output_get_2 (Variables|Cache|SetM_Tracks _returnvalue_4))
              (Rendering|Material|SetMaterial (Variables|Default|GetMesh) _returnvalue_2 _output_get_2)
              (CallFunction|RepaintRobotColor))))))
    (:then_3
      (Variables|Cache|SetTargetArmLen (Variables|/Script/Engine.SpringArmComponent|GetTargetArmLength (Variables|Default|GetSpringArm))))))

(fn GetMovementVector
  (bind _returnvalue (Transformation|GetActorLocation))
  (bind _returnvalue_2 (+ _returnvalue "0, 0, 0"))
  (bind _outhit (Class|KismetSystemLibrary|BoxTraceSingleforObjects _returnvalue_2 (+ _returnvalue_2 "0, 0,-300.000000") "60.000000,60.000000,1.000000" "0, 0, 0" (Utilities|Array|MakeArray "ObjectTypeQuery1" "ObjectTypeQuery2") false (Utilities|Array|MakeArray self) "None" true))
  (return (Math|Vector|Lerp(Vector) (* (Math|Vector|GetRightVector (Transformation|GetActorRotation)) -1.0) (Math|Vector|CrossProduct (.Normal (Collision|BreakHitResult _outhit)) (Math|Vector|GetUpVector (Transformation|GetActorRotation))) 0.5)))

(fn RepaintRobotColor
  (Rendering|Material|SetVectorParameterValue (Variables|Cache|GetM_Main) "Color" (Variables|Const|GetRobotColor) :!class /Script/Engine.MaterialInstanceDynamic))

(fn GetRootMesh
  (bind _asprimitive_component (Utilities|Casting|CastToPrimitiveComponent (VehicleSound|GetRootComponent))
    (:then
      _)
    (:CastFailed
      _))
  (return _asprimitive_component))

(fn DrawDebugVector
  (params (V :type Vector))
  (Rendering|Debug|DrawDebugLine (Transformation|GetActorLocation) V "(R=0.989000,G=0.000000,B=0.007870,A=1.000000)" 0.1 1.5))