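; MAARS projectile actor that deals damage and a physical push to the first actor it overlaps, then destroys itself.
; Overlap runs the projectile effect, then the visual effect, then destruction.
; The projectile effect applies damage credited to the owner and its instigator's controller, then adds an impulse to the target's root primitive along the projectile's forward vector.
; The visual effect is only a short-lived debug point at the impact location.
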(event Custom|ApplyVisualEffect
  (Rendering|Debug|DrawDebugPoint (Transformation|GetActorLocation) 1e+01 "(R=1.000000,G=0.062529,B=0.000000,A=1.000000)" 3.0))

(event Custom|ApplyProjectileEffect
  (params (Other :type Actor%20Object%20Reference))
  (Game|Damage|ApplyDamage Other (Variables|Default|GetDamage) (Game|GetInstigatorController (Components|GetOwner)) (Components|GetOwner) (Variables|Default|GetDamageTypeClass))
  (bind _asprimitive_component (Utilities|Casting|CastToPrimitiveComponent (VehicleSound|GetRootComponent Other)))
  (Utilities|IsValid _asprimitive_component
    (:Is%20Valid
      (Physics|AddImpulseatLocation _asprimitive_component (* (Math|Rotator|GetRotationXVector (Transformation|GetActorRotation)) (Variables|Default|GetImpulse)) (Transformation|GetActorLocation) "None"))))

(event EventBeginPlay)

(event Collision|EventActorBeginOverlap
  (params (OtherActor :type Actor%20Object%20Reference))
  (Utilities|FlowControl|Sequence
    (:then_0
      (CallFunction|ApplyProjectileEffect OtherActor))
    (:then_1
      (CallFunction|ApplyVisualEffect))
    (:then_2
      (Actor|DestroyActor))))

(event EventTick
  (params (DeltaSeconds :type Float%20%28single-precision%29)))

(fn ConstructionScript)